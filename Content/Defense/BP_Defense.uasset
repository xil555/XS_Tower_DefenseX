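; BP_Defense is a destructible turret that automatically fires BP_Bullet at Enemy-tagged actors inside its DetectionRange sphere.
; A looping Shoot timer reacquires lost targets from overlaps, while newly entering enemies immediately become the current target.
; A fast look timer turns the mesh's yaw toward the target.
; TakeDamage updates the health widget and destroys the turret at zero; BeginPlay briefly delays, then toggles detection collision.
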(event `Shoot`
  (bind _detectionrange (`self.detectionRange`))
  (if (not (and (`KismetSystemLibrary.IsValid` (`self.CurrentTarget`)) (`PrimitiveComponent.IsOverlappingActor` _detectionrange (`self.CurrentTarget`))))
    (set `self.CurrentTarget` null)
    (for _array_element (`PrimitiveComponent.GetOverlappingActors` _detectionrange null)
      (if (`self.ActorHasTag` _array_element "Enemy")
        (set `self.CurrentTarget` _array_element))))
  (`/Engine/EditorBlueprintResources/StandardMacros.IsValid` (`self.CurrentTarget`)
    (:`Is Valid`
      (`|SpawnActorFromClass` "/Game/Defense/BP_Bullet.BP_Bullet_C" (`SceneComponent.K2_GetComponentToWorld` (`self.Bullet`)) "AlwaysSpawn" "SelectDefaultAtRuntime" null null))))

(event `TakeDamage`
  (params (Amount :type "Float (double-precision)"))
  (set `self.CurrentHealth` (- (`self.CurrentHealth`) Amount))
  (bind _aswbp_defense_health (cast `/Game/UI/WBP_DefenseHealth` (`WidgetComponent.GetUserWidgetObject` (`self.HealthWidget`))))
  (`/Game/UI/WBP_DefenseHealth.SetHealthPercent` _aswbp_defense_health (/ (`self.CurrentHealth`) (`self.MaxHealth`)))
  (if (<= (`self.CurrentHealth`) 0.0)
    (`KismetSystemLibrary.K2_ClearAndInvalidateTimerHandle` (`self.TimerLookAt`))
    (`self.K2_DestroyActor`)))

(event `self.ReceiveBeginPlay`
  (bind _detectionrange (`self.detectionRange`))
  (set `self.CurrentHealth` (`self.MaxHealth`))
  (bind _returnvalue (`KismetSystemLibrary.K2_SetTimerDelegate` (delegate `Shoot`) 1.0 true))
  (`KismetSystemLibrary.K2_SetTimerDelegate` (delegate `LookTimer`) 0.03 true)
  (`KismetSystemLibrary.Delay` 0.2)
  (bind _aswbp_defense_health (cast `/Game/UI/WBP_DefenseHealth` (`WidgetComponent.GetUserWidgetObject` (`self.HealthWidget`))))
  (`/Game/UI/WBP_DefenseHealth.SetHealthPercent` _aswbp_defense_health 1.0)
  (`KismetSystemLibrary.Delay` 0.2)
  (`PrimitiveComponent.SetCollisionEnabled` _detectionrange "NoCollision")
  (`PrimitiveComponent.SetCollisionEnabled` _detectionrange "QueryOnly"))

(event `AcquireNextTarget`)

(event `LookingAtTarget`
  (params (Actor :type "Actor Object Reference"))
  (if (`self.ActorHasTag` Actor "Enemy")
    (set `self.CurrentTarget` Actor)
    (bind _returnvalue (`KismetSystemLibrary.K2_SetTimerDelegate` (delegate `LookTimer`) 0.03 true))
    (set `self.TimerLookAt` _returnvalue)))

(event `LookTimer`
  (bind _currenttarget (`self.CurrentTarget`))
  (bind (_returnvalue_roll _returnvalue_pitch _returnvalue_yaw) (`KismetMathLibrary.BreakRotator` (`KismetMathLibrary.FindLookAtRotation` (`self.K2_GetActorLocation`) (`self.K2_GetActorLocation` _currenttarget))))
  (`/Engine/EditorBlueprintResources/StandardMacros.IsValid` _currenttarget
    (:`Is Valid`
      (`SceneComponent.K2_SetWorldRotation` (`self.StaticMesh`) (`KismetMathLibrary.MakeRotator` 0.0 0.0 _returnvalue_yaw) false false))))

(event `self.detectionRange.OnComponentBeginOverlap`
  (params (OverlappedComponent :type "PrimitiveComponent Object Reference") (OtherActor :type "Actor Object Reference") (OtherComp :type "PrimitiveComponent Object Reference") (OtherBodyIndex :type Integer) (bFromSweep :type Boolean) (SweepResult :type "HitResult Structure (by ref)"))
  ; Zone Where Defense looks at you and fire
  (`/Engine/EditorBlueprintResources/StandardMacros.IsValid` OtherActor
    (:`Is Valid`
      (if (`self.ActorHasTag` OtherActor "Enemy")
        (`self.LookingAtTarget` OtherActor)))))

(event `self.detectionRange.OnComponentEndOverlap`
  (params (OverlappedComponent :type "PrimitiveComponent Object Reference") (OtherActor :type "Actor Object Reference") (OtherComp :type "PrimitiveComponent Object Reference") (OtherBodyIndex :type Integer))
  ; Zone Where Defense looks at you and fire
)

(fn `ReceiveDamage `)

(fn `UserConstructionScript`
  (`SphereComponent.SetSphereRadius` (`self.detectionRange`) (`self.In Sphere Radius`) true))
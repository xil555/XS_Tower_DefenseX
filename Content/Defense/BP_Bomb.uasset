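; BP_Bomb is a projectile actor that flies forward at constant speed and kills the first recognised enemy it touches.
; Tick moves it with a swept offset, and its sphere overlap casts Enemy-tagged actors to Mummy, Archer or SandWorm, calls Die, then destroys the bomb.
; An Explode event deals heavy radius damage to tagged enemies, but nothing connected here calls it, and the BeginPlay delay leads nowhere.
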(event `self.ReceiveBeginPlay`
  (`KismetSystemLibrary.Delay` 1.0))

(event `self.ReceiveTick`
  (params (DeltaSeconds :type "Float (single-precision)"))
  (`self.K2_AddActorWorldOffset` (* (`self.GetActorForwardVector`) 900.0 DeltaSeconds) true))

(event `Explode`
  (bind _outactors (`GameplayStatics.GetAllActorsOfClassWithTag` null "Enemy"))
  (for _array_element _outactors
    (if (<= (`self.GetDistanceTo` _array_element) 1000.0)
      (`GameplayStatics.ApplyDamage` _array_element 999.0)))
  (`self.K2_DestroyActor`))

(event `self.Sphere.OnComponentBeginOverlap`
  (params (OverlappedComponent :type "PrimitiveComponent Object Reference") (OtherActor :type "Actor Object Reference") (OtherComp :type "PrimitiveComponent Object Reference") (OtherBodyIndex :type Integer) (bFromSweep :type Boolean) (SweepResult :type "HitResult Structure (by ref)"))
  (if (`self.ActorHasTag` OtherActor "Enemy")
    (bind _asbp_mummy (cast `/Game/Blueprints/BP_Mummy` OtherActor)
      (:`then`
        (`/Game/Blueprints/BP_Mummy.Die` _asbp_mummy)
        (`self.K2_DestroyActor`))
      (:`CastFailed`
        (bind _asbp_archer (cast `/Game/Blueprints/BP_Archer` OtherActor)
          (:`then`
            (`/Game/Blueprints/BP_Archer.Die` _asbp_archer)
            (`self.K2_DestroyActor`))
          (:`CastFailed`
            (bind _asbp_sand_worm (cast `/Game/Blueprints/BP_SandWorm` OtherActor))
            (`/Game/Blueprints/BP_SandWorm.Die` _asbp_sand_worm)
            (`self.K2_DestroyActor`)))))))

(fn `UserConstructionScript`)
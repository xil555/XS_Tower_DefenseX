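; Projectile for the defense game that freezes the first supported enemy it hits.
; Tick moves it forward at constant speed with a swept world offset.
; Sphere overlap checks the Enemy tag, casts in turn to Mummy, SandWorm or Archer, calls FreezeEnemy and destroys the bullet.
; The empty Explode event, disconnected area-damage chains and dangling BeginPlay delay have no effect.
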(event `self.ReceiveBeginPlay`
  (`KismetSystemLibrary.Delay` 1.0))

(event `self.ReceiveTick`
  (params (DeltaSeconds :type "Float (single-precision)"))
  (`self.K2_AddActorWorldOffset` (* DeltaSeconds (* (`self.GetActorForwardVector`) 1500.0)) true))

(event `Explode`)

(event `self.Sphere.OnComponentBeginOverlap`
  (params (OverlappedComponent :type "PrimitiveComponent Object Reference") (OtherActor :type "Actor Object Reference") (OtherComp :type "PrimitiveComponent Object Reference") (OtherBodyIndex :type Integer) (bFromSweep :type Boolean) (SweepResult :type "HitResult Structure (by ref)"))
  (if (`self.ActorHasTag` OtherActor "Enemy")
    (bind _asbp_mummy (cast `/Game/Blueprints/BP_Mummy` OtherActor)
      (:`then`
        (`/Game/Blueprints/BP_Mummy.FreezeEnemy` _asbp_mummy)
        (`self.K2_DestroyActor`))
      (:`CastFailed`
        (bind _asbp_sand_worm (cast `/Game/Blueprints/BP_SandWorm` OtherActor)
          (:`then`
            (`/Game/Blueprints/BP_SandWorm.FreezeEnemy` _asbp_sand_worm)
            (`self.K2_DestroyActor`))
          (:`CastFailed`
            (bind _asbp_archer (cast `/Game/Blueprints/BP_Archer` OtherActor))
            (`/Game/Blueprints/BP_Archer.FreezeEnemy` _asbp_archer)
            (`self.K2_DestroyActor`)))))))

(fn `UserConstructionScript`)
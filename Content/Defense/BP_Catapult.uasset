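; Defensive catapult that automatically targets and fires at Enemy-tagged actors, and is destroyed when its health runs out.
; A DetectionRange sphere and overlap scans pick targets, then looping timers turn its yaw toward the target and spawn BP_Bullet at FireRate.
; Two damage handlers, TakeDamage and ReceiveDamage, update the health bar widget.
; UpgradeCatapult adds health and swaps the mesh material by level; its fire-rate boost is disconnected.
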(event `TakeDamage`
  (params (Amount :type "Float (double-precision)"))
  (set `self.CurrentHealth` (- (`self.CurrentHealth`) Amount))
  (bind _aswbp_bomb_health_1 (cast `/Game/UI/WBP_BombHealth1` (`WidgetComponent.GetUserWidgetObject` (`self.HealthWidget`))))
  (`/Game/UI/WBP_BombHealth1.SetHealthPercent` _aswbp_bomb_health_1 (/ (`self.CurrentHealth`) (`self.MaxHealth`)))
  (if (<= (`self.CurrentHealth`) 0.0)
    (`KismetSystemLibrary.K2_ClearAndInvalidateTimerHandle` (`self.TimerLookAt`))
    (`self.K2_DestroyActor`)))

(event `self.ReceiveBeginPlay`
  (set `self.CurrentHealth` (`self.MaxHealth`))
  (`KismetSystemLibrary.Delay` 0.1)
  (`self.AcquireNextTarget`))

(event `AcquireNextTarget`
  (`/Engine/EditorBlueprintResources/StandardMacros.IsValid` (`self.CurrentTarget`)
    (:`Is Not Valid`
      (for _array_element (`self.GetOverlappingActors` (`ActorComponent.GetOwner` (`self.detectionRange`)) null)
        (if (`self.ActorHasTag` _array_element "Enemy")
          (if (<= (`KismetMathLibrary.Vector_Distance` (`self.K2_GetActorLocation`) (`self.K2_GetActorLocation` _array_element)) 1000.0)
            (set `self.CurrentTarget` _array_element)
            (bind _returnvalue (`KismetSystemLibrary.K2_SetTimerDelegate` (delegate `LookTimer`) 0.05 true))
            (set `self.TimerLookAt` _returnvalue)
            (bind _returnvalue_2 (`KismetSystemLibrary.K2_SetTimerDelegate` (delegate `ShootBomb`) (`self.FireRate `) true))
            (set `self.TimerBomb` _returnvalue_2)
            (for _ (range 1)
              _)))))))

(event `ShootBomb`
  (`/Engine/EditorBlueprintResources/StandardMacros.IsValid` (`self.CurrentTarget`)
    (:`Is Valid`
      (`|SpawnActorFromClass` "/Game/Defense/BP_Bullet.BP_Bullet_C" (`SceneComponent.K2_GetComponentToWorld` (`self.Bullet`)) "AlwaysSpawn" "MultiplyWithRoot" null null))))

(event `LookingAtTarget`
  (params (Actor :type "Actor Object Reference"))
  (if (`self.ActorHasTag` Actor "Enemy")
    (if (<= (`KismetMathLibrary.Vector_Distance` (`self.K2_GetActorLocation`) (`self.K2_GetActorLocation` Actor)) 1000.0)
      (bind _output_get (set `self.CurrentTarget` Actor))
      (bind _returnvalue (`KismetSystemLibrary.K2_SetTimerDelegate` (delegate `LookTimer`) 0.3 true))
      (set `self.TimerLookAt` _returnvalue)
      (bind _returnvalue_2 (`KismetSystemLibrary.K2_SetTimerDelegate` (delegate `ShootBomb`) (`self.FireRate `) true))
      (set `self.TimerBomb` _returnvalue_2))))

(event `LookTimer`
  (bind _returnvalue (`self.K2_GetActorLocation`))
  (bind (_returnvalue_roll _returnvalue_pitch _returnvalue_yaw) (`KismetMathLibrary.BreakRotator` (`KismetMathLibrary.FindLookAtRotation` _returnvalue (`self.K2_GetActorLocation` (`self.CurrentTarget`)))))
  (`/Engine/EditorBlueprintResources/StandardMacros.IsValid` (stale `LookingAtTarget` _output_get)
    (:`Is Valid`
      (if (<= (`KismetMathLibrary.Vector_Distance` (`self.K2_GetActorLocation` (`self.CurrentTarget`)) _returnvalue) 2000.0)
        (`self.K2_SetActorRotation` (`KismetMathLibrary.MakeRotator` 0.0 0.0 _returnvalue_yaw))
        (else
          (set `self.CurrentTarget` null))))
    (:`Is Not Valid`
      (`self.AcquireNextTarget`))))

(event `self.detectionRange.OnComponentBeginOverlap`
  (params (OverlappedComponent :type "PrimitiveComponent Object Reference") (OtherActor :type "Actor Object Reference") (OtherComp :type "PrimitiveComponent Object Reference") (OtherBodyIndex :type Integer) (bFromSweep :type Boolean) (SweepResult :type "HitResult Structure (by ref)"))
  ; Zone Where Defense looks at you and fire
  (`self.LookingAtTarget` OtherActor))

(event `self.detectionRange.OnComponentEndOverlap`
  (params (OverlappedComponent :type "PrimitiveComponent Object Reference") (OtherActor :type "Actor Object Reference") (OtherComp :type "PrimitiveComponent Object Reference") (OtherBodyIndex :type Integer))
  ; Zone Where Defense looks at you and fire
  (if (== OtherActor (`self.CurrentTarget`))
    (`KismetSystemLibrary.K2_ClearAndInvalidateTimerHandle` (`self.TimerBomb`))
    (set `self.TimerBomb` (struct))
    (set `self.CurrentTarget` null)
    (`self.AcquireNextTarget`)))

(fn `ReceiveDamage `
  (params (Amount :type "Float (double-precision)"))
  (set `self.CurrentHealth` (- (`self.CurrentHealth`) Amount))
  (bind _aswbp_bomb_health_1 (cast `/Game/UI/WBP_BombHealth1` (`WidgetComponent.GetUserWidgetObject` (`self.HealthWidget`))))
  (`/Game/UI/WBP_BombHealth1.SetHealthPercent` _aswbp_bomb_health_1 (/ (`self.CurrentHealth`) (`self.MaxHealth`)))
  (if (<= (`self.CurrentHealth`) 0.0)
    (`self.K2_DestroyActor`)))

(fn `UpgradeCatapult`
  (bind _upgradelevel (`self.UpgradeLevel`))
  (set `self.MaxHealth` (+ (`self.MaxHealth`) 150.0))
  (set `self.CurrentHealth` (+ (`self.CurrentHealth`) 150.0))
  (set `self.UpgradeLevel` (+ _upgradelevel 1))
  (if (== _upgradelevel 1)
    (`PrimitiveComponent.SetMaterial` (`self.StaticMesh`) 0 (`self.M_Catapult_L1`))
    (else
      (`PrimitiveComponent.SetMaterial` (`self.StaticMesh`) 0 (`self.M_Catapult_L2`)))))

(fn `UserConstructionScript`
  (`SphereComponent.SetSphereRadius` (`self.detectionRange`) (`self.In Sphere Radius`) true))
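; Freeze defense actor that spawns a BP_FreezeBullet every ten seconds and destroys itself when its health, shown on a widget, runs out.
; Shortly after BeginPlay it runs one pulse calling FreezeEnemy on Mummy, SandWorm and Archer enemies inside its detection sphere.
; LookingAtTarget starts a timer that yaws the actor toward a target.
; Range overlap events call AcquireNextTarget, which is empty, leaving nearest-enemy selection logic disconnected.
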(event `Shoot`
  (`|SpawnActorFromClass` "/Game/Defense/BP_FreezeBullet.BP_FreezeBullet_C" (`self.GetTransform`) "AlwaysSpawn" "MultiplyWithRoot" null null))

(event `TakeDamage`
  (params (Amount :type "Float (double-precision)"))
  (set `self.CurrentHealth_0` (- (`self.CurrentHealth_0`) Amount))
  (bind _aswbp_freeze_health_2 (cast `/Game/UI/WBP_FreezeHealth2` (`WidgetComponent.GetUserWidgetObject` (`self.Widget`))))
  (`/Game/UI/WBP_FreezeHealth2.SetHealthPercent` _aswbp_freeze_health_2 (/ (`self.CurrentHealth_0`) (`self.MaxHealth_0`)))
  (if (<= (`self.CurrentHealth_0`) 0.0)
    (`KismetSystemLibrary.K2_ClearAndInvalidateTimerHandle` (`self.TimerLookAt_0`))
    (`self.K2_DestroyActor`)))

(event `self.ReceiveBeginPlay`
  (set `self.CurrentHealth_0` (`self.MaxHealth_0`))
  (`KismetSystemLibrary.Delay` 0.1)
  (`KismetSystemLibrary.K2_SetTimerDelegate` (delegate `Shoot`) 10.0 true)
  (`self.DoFreezePulse `))

(event `AcquireNextTarget`)

(event `LookingAtTarget`
  (params (Actor :type "Actor Object Reference"))
  (set `self.CurrentTarget_0` Actor)
  (`KismetSystemLibrary.K2_ClearAndInvalidateTimerHandle` (`self.TimerLookAt_0`))
  (bind _returnvalue (`KismetSystemLibrary.K2_SetTimerDelegate` (delegate `LookTimer`) 0.5 true))
  (set `self.TimerLookAt_0` _returnvalue))

(event `LookTimer`
  (bind _currenttarget_0 (`self.CurrentTarget_0`))
  (bind (_returnvalue_roll _returnvalue_pitch _returnvalue_yaw) (`KismetMathLibrary.BreakRotator` (`KismetMathLibrary.FindLookAtRotation` (`self.K2_GetActorLocation`) (`self.K2_GetActorLocation` _currenttarget_0))))
  (`/Engine/EditorBlueprintResources/StandardMacros.IsValid` _currenttarget_0
    (:`Is Valid`
      (`self.K2_SetActorRotation` (`KismetMathLibrary.MakeRotator` 0.0 0.0 _returnvalue_yaw)))
    (:`Is Not Valid`
      (`self.AcquireNextTarget`))))

(event `self.detectionRange_0.OnComponentBeginOverlap`
  (params (OverlappedComponent :type "PrimitiveComponent Object Reference") (OtherActor :type "Actor Object Reference") (OtherComp :type "PrimitiveComponent Object Reference") (OtherBodyIndex :type Integer) (bFromSweep :type Boolean) (SweepResult :type "HitResult Structure (by ref)"))
  ; Zone Where Defense looks at you and fire
  (`/Engine/EditorBlueprintResources/StandardMacros.IsValid` OtherActor
    (:`Is Valid`
      (if (`self.ActorHasTag` OtherActor "Enemy")
        (`self.AcquireNextTarget` :!label _label)))))

(event `self.detectionRange_0.OnComponentEndOverlap`
  (params (OverlappedComponent :type "PrimitiveComponent Object Reference") (OtherActor :type "Actor Object Reference") (OtherComp :type "PrimitiveComponent Object Reference") (OtherBodyIndex :type Integer))
  ; Zone Where Defense looks at you and fire
  (`/Engine/EditorBlueprintResources/StandardMacros.IsValid` OtherActor
    (:`Is Valid`
      (if (== OtherActor (`self.CurrentTarget_0`))
        (`KismetSystemLibrary.K2_ClearAndInvalidateTimerHandle` (`self.TimerLookAt_0`))
        (set `self.TimerLookAt_0` (struct))
        (set `self.CurrentTarget_0` null)
        (goto _label)))))

(event `DoFreezePulse`
  (if (not (`self.CanFreeze`))
    (set `self.CanFreeze` false)
    (for _array_element (`PrimitiveComponent.GetOverlappingActors` (`self.detectionRange_0`) null)
      (if (`self.ActorHasTag` _array_element "Enemy")
        (bind _asbp_mummy (cast `/Game/Blueprints/BP_Mummy` _array_element)
          (:`then`
            (`/Game/Blueprints/BP_Mummy.FreezeEnemy` _asbp_mummy))
          (:`CastFailed`
            (bind _asbp_sand_worm (cast `/Game/Blueprints/BP_SandWorm` _array_element)
              (:`then`
                (`/Game/Blueprints/BP_SandWorm.FreezeEnemy` _asbp_sand_worm))
              (:`CastFailed`
                (bind _asbp_archer (cast `/Game/Blueprints/BP_Archer` _array_element))
                (`/Game/Blueprints/BP_Archer.FreezeEnemy` _asbp_archer)))))))
    (`KismetSystemLibrary.Delay` (`self.FreezeDuration`))
    (`KismetSystemLibrary.Delay` (`self.FreezeCooldown`))
    (set `self.CanFreeze` true)))

(fn `UserConstructionScript`
  (`SphereComponent.SetSphereRadius` (`self.detectionRange_0`) (`self.In Sphere Radius_0`) true))
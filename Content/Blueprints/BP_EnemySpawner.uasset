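; Enemy spawner that sends mummies, archers and sand worms at the tower along one of three random paths from BP_World.
; A self-rescheduling timer spawns one enemy per cycle and passes it the path points and tower reference.
; Tick advances the wave on a fixed clock, shortening the spawn delay down to a minimum and shifting type weights from mummy-only toward a mixed roster.
; Weighted selection uses separate random rolls per branch; disconnected popup-widget code never runs.
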(event `SpawnMummy`
  (bind _mummyweight (`self.MummyWeight`))
  (bind _world (`self.World`))
  (bind _returnvalue (`KismetMathLibrary.Conv_VectorToTransform` (`|GetArrayItem` (`self.ChosenPoints`))))
  (bind _returnvalue_2 (`KismetMathLibrary.RandomIntegerInRange` 0 (- (+ (`self.MummyWeight`) (`self.ArcherWeight`) (`self.WormWeight`)) 1)))
  (if (`self.bActive`)
    (set `self.NextDelay` (- (`self.BaseDelay`) (* (- (`self.WaveIndex`) 1) (`self.DelayStep`))))
    (if (< (`self.NextDelay`) (`self.MinDelay`))
      (set `self.NextDelay` (`self.MinDelay`)))
    (if (<= (`self.WaveIndex`) 2)
      (set `self.MummyWeight` 100)
      (set `self.ArcherWeight` 0)
      (set `self.WormWeight` 0)
      (elif (<= (`self.WaveIndex`) 4)
        (set `self.MummyWeight` 70)
        (set `self.ArcherWeight` 15)
        (set `self.WormWeight` 15)
        (else
          (set `self.MummyWeight` 50)
          (set `self.ArcherWeight` 25)
          (set `self.WormWeight` 25))))
    (`/Engine/EditorBlueprintResources/StandardMacros.IsValid` _world
      (:`Is Valid`
        (switch `int` (`KismetMathLibrary.RandomIntegerInRange` 0 2)
          (:`0`
            (set `self.ChosenPoints` (`/Game/Blueprints/BP_World.Path1` _world)))
          (:`1`
            (set `self.ChosenPoints` (`/Game/Blueprints/BP_World.Path2` _world)))
          (:`2`
            (set `self.ChosenPoints` (`/Game/Blueprints/BP_World.Path3` _world))))
        (set `self.Spawn Xform` _returnvalue)
        (if (< _returnvalue_2 _mummyweight)
          (bind _returnvalue_3 (`|SpawnActorFromClass` (`self.MummyClass`) _returnvalue "AlwaysSpawn" "MultiplyWithRoot" null null))
          (bind _asbp_mummy (cast `/Game/Blueprints/BP_Mummy` _returnvalue_3))
          (`/Game/Blueprints/BP_Mummy.SetupMummy` _asbp_mummy (`self.ChosenPoints`) (`/Game/Blueprints/BP_World.TowerRef` (`self.World`)))
          (elif (< _returnvalue_2 (+ _mummyweight (`self.ArcherWeight`)))
            (bind _returnvalue_4 (`|SpawnActorFromClass` (`self.ArcherClass`) _returnvalue "AlwaysSpawn" "MultiplyWithRoot" null null))
            (bind _asbp_archer (cast `/Game/Blueprints/BP_Archer` _returnvalue_4))
            (`/Game/Blueprints/BP_Archer.SetupArcher` _asbp_archer (`self.ChosenPoints`) (`/Game/Blueprints/BP_World.TowerRef` (`self.World`)))
            (else
              (bind _returnvalue_5 (`|SpawnActorFromClass` (`self.WormClass`) _returnvalue "AlwaysSpawn" "MultiplyWithRoot" null null))
              (bind _asbp_sand_worm (cast `/Game/Blueprints/BP_SandWorm` _returnvalue_5))
              (`/Game/Blueprints/BP_SandWorm.SetupWorm` _asbp_sand_worm (`self.ChosenPoints`) (`/Game/Blueprints/BP_World.TowerRef` (`self.World`))))))
        (`KismetSystemLibrary.K2_SetTimerDelegate` (delegate `SpawnMummy`) (`self.NextDelay`))))))

(event `self.ReceiveTick`
  (params (DeltaSeconds :type "Float (single-precision)"))
  (bind _waveclock (`self.WaveClock`))
  (set `self.WaveClock` (+ DeltaSeconds _waveclock))
  (if (>= _waveclock (`self.WaveLength`))
    (set `self.WaveIndex` (+ (`self.WaveIndex`) 1))
    (set `self.WaveClock` 0.0)))

(event `self.ReceiveBeginPlay`
  (set `self.bActive` true)
  (bind _returnvalue (`GameplayStatics.GetActorOfClass` "/Game/Blueprints/BP_World.BP_World_C"))
  (set `self.World` _returnvalue)
  (`KismetSystemLibrary.Delay` 0.5)
  (`self.SpawnMummy`))

(fn `UserConstructionScript`)
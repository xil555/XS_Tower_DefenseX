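; BP_Tower is the tower actor whose health decides game over, shown through its own health widget.
; ReceiveDamage applies scaled damage, refreshes the player HUD's shop and health bar, and opens the game-over screen at zero health.
; RegisterKill spawns a gem at the kill location every KillsPerGem kills.
; UpgradeTower spends gems on two tiers that add health, reveal pieces and swap materials, the second also reducing damage taken.
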(event `self.ReceiveBeginPlay`
  (bind _returnvalue (`|CreateWidget` "/Game/UI/W_TowerHealth.W_TowerHealth_C"))
  (bind _output_get (set `self.TowerHealthWidget` _returnvalue))
  (`UserWidget.AddToViewport` _output_get 0)
  (`/Game/UI/W_TowerHealth.SetHealthPercent ` _output_get 1.0 (`self.CurrentHealth`) (`self.MaxHealth`)))

(fn `ReceiveDamage`
  (params (Amount :type "Float (double-precision)"))
  (bind _returnvalue (`GameplayStatics.GetPlayerController` 0))
  (bind _maxhealth (`self.MaxHealth`))
  (bind _output_get (set `self.CurrentHealth` (- (`self.CurrentHealth`) (* Amount (`self.DamageTakenScale`)))))
  (bind _asbp_player_pawn (cast `/Game/Blueprints/BP_PlayerPawn` (`GameplayStatics.GetPlayerPawn` 0)))
  (bind _hudref (`/Game/Blueprints/BP_PlayerPawn.HUDRef` _asbp_player_pawn))
  (`/Game/UI/W_HUD.RefreshShop` _hudref)
  (`/Engine/EditorBlueprintResources/StandardMacros.IsValid` _hudref
    (:`Is Valid`
      (`/Game/UI/W_TowerHealth.SetHealthPercent ` (`self.TowerHealthWidget`) (/ _output_get _maxhealth) (`self.CurrentHealth`) _maxhealth)
      (if (<= (`self.CurrentHealth`) 0.0)
        (set `self.bDead` true)
        (bind _returnvalue_2 (`|CreateWidget` "/Game/UI/W_GameOver.W_GameOver_C"))
        (`UserWidget.AddToViewport` _returnvalue_2 0)
        (set `PlayerController.bShowMouseCursor` true _returnvalue)
        (`WidgetBlueprintLibrary.SetInputMode_UIOnlyEx` _returnvalue null)))))

(fn `RegisterKill`
  (params (SpawnLocation :type "Vector Structure"))
  (set `self.KillCount` (+ (`self.KillCount`) 1))
  (if (>= (`self.KillCount`) (`self.KillsPerGem`))
    (set `self.KillCount` 0)
    (`|SpawnActorFromClass` (`self.GemClass`) (`KismetMathLibrary.MakeTransform` (+ SpawnLocation (`KismetMathLibrary.MakeVector` 0.0 0.0 80.0))) "AlwaysSpawn" "MultiplyWithRoot" null null)
    (`KismetSystemLibrary.PrintText` "Gem Spawned")))

(fn `UpgradeTower`
  (locals (Cost :type Integer))
  (bind _upgradelevel (`self.UpgradeLevel`))
  (bind _towerhealthwidget (`self.TowerHealthWidget`))
  (bind _returnvalue (- (`self.Gems`) (`local.Cost`)))
  (`KismetSystemLibrary.PrintString` "clicked")
  (if (>= _upgradelevel 2)
    _
    (elif (== _upgradelevel 0)
      (set `local.Cost` (`self.Upgrade1Cost`))
      (if (>= (`self.Gems`) (`local.Cost`))
        (set `self.Gems` _returnvalue)
        (set `self.UpgradeLevel` (+ (`self.UpgradeLevel`) 1) :!label _label)
        (bind _output_get (set `self.MaxHealth` (+ (`self.MaxHealth`) 400.0)))
        (`KismetSystemLibrary.PrintString` (`KismetStringLibrary.Conv_DoubleToString` _output_get))
        (bind _output_get_2 (set `self.CurrentHealth` (+ (`self.CurrentHealth`) 400.0)))
        (`KismetSystemLibrary.PrintString` (`KismetStringLibrary.Conv_DoubleToString` _output_get_2))
        (`/Game/UI/W_TowerHealth.SetHealthPercent ` _towerhealthwidget (/ (`self.CurrentHealth`) (`self.MaxHealth`)) _output_get_2 _output_get)
        (`/Game/UI/W_TowerHealth.SetHealthNumbers` _towerhealthwidget (`|FormatText` "{Current} / {Max}" _output_get_2 _output_get))
        (if (== (`self.UpgradeLevel`) 1)
          (`SceneComponent.SetHiddenInGame` (`self.UpgradePiece1`) false false)
          (`PrimitiveComponent.SetMaterial` (`self.UpgradePiece1`) 0 (`self.MatLevel1`))
          (`PrimitiveComponent.SetMaterial` (`self.Tower`) 0 (`self.MatLevel1`))
          (else
            (`SceneComponent.SetHiddenInGame` (`self.UpgradePiece2`) false false)
            (`PrimitiveComponent.SetMaterial` (`self.UpgradePiece2`) 0 (`self.MatLevel2`))
            (`PrimitiveComponent.SetMaterial` (`self.Tower`) 0 (`self.MatLevel2`))
            (`PrimitiveComponent.SetMaterial` (`self.UpgradePiece1`) 0 (`self.MatLevel2`))))
        (if (== (`self.UpgradeLevel`) 2)
          (set `self.DamageTakenScale` 0.75))
        (bind _asbp_player_pawn (cast `/Game/Blueprints/BP_PlayerPawn` (`GameplayStatics.GetPlayerPawn` 0)))
        (`/Game/UI/W_HUD.RefreshShop` (`/Game/Blueprints/BP_PlayerPawn.HUDRef` _asbp_player_pawn)))
      (else
        (set `local.Cost` (`self.Upgrade2Cost`))
        (if (>= (`self.Gems`) (`local.Cost`))
          (set `self.Gems` _returnvalue)
          (goto _label))))))

(fn `UserConstructionScript`)
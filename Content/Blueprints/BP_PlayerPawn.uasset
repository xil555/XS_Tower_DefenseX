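; Player pawn for a tower defense game that creates the HUD and handles mouse-driven defense placement.
; Keys 1-3 select catapult, bomb or freeze cannon, and Tick moves a green/red ghost mesh to the cursor trace.
; Clicks spawn defenses away from the tower and within a distance band of three enemy paths, spending placements and BP_Tower stock.
; RegisterKill grants the tower a gem every second kill.
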(event `self.ReceiveBeginPlay`
  (bind _hudref (`self.HUDRef`))
  (set `PlayerController.bShowMouseCursor` true (`GameplayStatics.GetPlayerController` 0))
  (bind _returnvalue (`|CreateWidget` "/Game/UI/W_HUD.W_HUD_C" (`GameplayStatics.GetPlayerController` 0)))
  (bind _output_get (set `self.HUDRef` _returnvalue))
  (`/Game/UI/W_HUD.SetDefenseLeft` _output_get (`self.DefensesLeft`))
  (`KismetSystemLibrary.Delay` 0.2)
  (`/Game/UI/W_HUD.SetSelectedSlot` (`self.HUDRef`) 0)
  (bind _returnvalue_2 (`GameplayStatics.GetActorOfClass` "/Game/Blueprints/BP_Tower.BP_Tower_C"))
  (`UserWidget.AddToViewport` _hudref 0)
  (set `/Game/UI/W_HUD.TowerRef` _returnvalue_2 _hudref)
  (`/Game/UI/W_HUD.RefreshShop` _hudref))

(event `Key|LeftMouseButton`
  (params (Key :type "Key Structure"))
  (:`Pressed`
    (bind (_returnvalue _outhit) (`self.Mouse Trace`))
    (if _returnvalue
      (if (> (`self.DefensesLeft`) 0)
        (bind _returnvalue_2 (`GameplayStatics.GetActorOfClass` "/Game/Blueprints/BP_Tower.BP_Tower_C"))
        (bind (_bblockinghit _binitialoverlap _time _distance _location _impactpoint _normal _impactnormal _physmat _hitactor) (`GameplayStatics.BreakHitResult` _outhit))
        (cast `/Game/Blueprints/BP_Tower` _hitactor
          (:`CastFailed`
            (cast `/Game/Defense/BP_Catapult` _hitactor
              (:`CastFailed`
                (cast `/Game/Defense/BP_FreezeCannon` _hitactor
                  (:`CastFailed`
                    (cast `/Game/Defense/BP_DefenseBomb` _hitactor
                      (:`CastFailed`
                        (if (> (`KismetMathLibrary.Vector_Distance` _location (`self.K2_GetActorLocation` _returnvalue_2)) 2500.0)
                          (set `self.ClosestPath` 99999.0)
                          (bind _returnvalue_3 (`GameplayStatics.GetActorOfClass` "/Game/Blueprints/BP_World.BP_World_C"))
                          (bind _path1 (`/Game/Blueprints/BP_World.Path1` _returnvalue_3))
                          (for (_array_element _array_index) _path1
                            (if (< _array_index (- (`KismetArrayLibrary.Array_Length` _path1) 1))
                              (bind _returnvalue_4 (`KismetMathLibrary.Distance2D` (`KismetMathLibrary.Conv_VectorToVector2D` _location) (`KismetMathLibrary.Conv_VectorToVector2D` (`KismetMathLibrary.FindClosestPointOnSegment` _location _array_element (`|GetArrayItem` _path1 (+ _array_index 1))))))
                              (if (< _returnvalue_4 (`self.ClosestPath`))
                                (set `self.ClosestPath` _returnvalue_4))))
                          (bind _path2 (`/Game/Blueprints/BP_World.Path2` _returnvalue_3))
                          (for (_array_element_2 _array_index_2) _path2
                            (if (< _array_index_2 (- (`KismetArrayLibrary.Array_Length` _path2) 1))
                              (bind _returnvalue_5 (`KismetMathLibrary.Distance2D` (`KismetMathLibrary.Conv_VectorToVector2D` _location) (`KismetMathLibrary.Conv_VectorToVector2D` (`KismetMathLibrary.FindClosestPointOnSegment` _location _array_element_2 (`|GetArrayItem` _path2 (+ _array_index_2 1))))))
                              (if (< _returnvalue_5 (`self.ClosestPath`))
                                (set `self.ClosestPath` _returnvalue_5))))
                          (bind _path3 (`/Game/Blueprints/BP_World.Path3` _returnvalue_3))
                          (for (_array_element_3 _array_index_3) _path3
                            (if (< _array_index_3 (- (`KismetArrayLibrary.Array_Length` _path3) 1))
                              (bind _returnvalue_6 (`KismetMathLibrary.Distance2D` (`KismetMathLibrary.Conv_VectorToVector2D` _location) (`KismetMathLibrary.Conv_VectorToVector2D` (`KismetMathLibrary.FindClosestPointOnSegment` _location _array_element_3 (`|GetArrayItem` _path3 (+ _array_index_3 1))))))
                              (if (< _returnvalue_6 (`self.ClosestPath`))
                                (set `self.ClosestPath` _returnvalue_6))))
                          (if (> (`self.ClosestPath`) 250.0)
                            (if (< (`self.ClosestPath`) 1200.0)
                              (bind _returnvalue_7 (`GameplayStatics.GetActorOfClass` "/Game/Blueprints/BP_Tower.BP_Tower_C"))
                              (switch `int` (`self.Selected Defense`)
                                (:`0`
                                  (if (> (`/Game/Blueprints/BP_Tower.StockCatapult` _returnvalue_7) 0)
                                    (switch `int` (`self.Selected Defense`) :!label _label
                                      (:`0`
                                        (bind _returnvalue_8 (`KismetMathLibrary.MakeRotFromZ` _impactnormal))
                                        (`|SpawnActorFromClass` "/Game/Defense/BP_Catapult.BP_Catapult_C" (`KismetMathLibrary.MakeTransform` _impactpoint _returnvalue_8 (2.0 2.0 2.0)) "AlwaysSpawn" "MultiplyWithRoot" null 3500.0 true 1.0 null))
                                      (:`1`
                                        (`|SpawnActorFromClass` "/Game/Defense/BP_DefenseBomb.BP_DefenseBomb_C" (`KismetMathLibrary.MakeTransform` _impactpoint _returnvalue_8 (2.0 2.0 2.0)) "AlwaysSpawn" "MultiplyWithRoot" null 3500.0 true 1.0 null))
                                      (:`2`
                                        (`|SpawnActorFromClass` "/Game/Defense/BP_FreezeCannon.BP_FreezeCannon_C" (`KismetMathLibrary.MakeTransform` _impactpoint _returnvalue_8 (2.0 2.0 2.0)) "AlwaysSpawn" "MultiplyWithRoot" null 3500.0 true 1.0 null)))
                                    (bind _output_get (set `self.DefensesLeft` (- (`self.DefensesLeft`) 1)))
                                    (`/Game/UI/W_HUD.SetDefenseLeft` (`self.HUDRef`) _output_get)
                                    (bind _returnvalue_9 (`GameplayStatics.GetActorOfClass` "/Game/Blueprints/BP_Tower.BP_Tower_C"))
                                    (switch `int` (`self.Selected Defense`)
                                      (:`0`
                                        (set `/Game/Blueprints/BP_Tower.StockCatapult` (- (`/Game/Blueprints/BP_Tower.StockCatapult` _returnvalue_9) 1) _returnvalue_9))
                                      (:`1`
                                        (set `/Game/Blueprints/BP_Tower.StockBomb` (- (`/Game/Blueprints/BP_Tower.StockBomb` _returnvalue_9) 1) _returnvalue_9))
                                      (:`2`
                                        (set `/Game/Blueprints/BP_Tower.StockFreeze` (- (`/Game/Blueprints/BP_Tower.StockFreeze` _returnvalue_9) 1) _returnvalue_9)))
                                    (`/Game/UI/W_HUD.RefreshShop` (`self.HUDRef`))))
                                (:`1`
                                  (if (> (`/Game/Blueprints/BP_Tower.StockBomb` _returnvalue_7) 0)
                                    (goto _label)))
                                (:`2`
                                  (if (> (`/Game/Blueprints/BP_Tower.StockFreeze` _returnvalue_7) 0)
                                    (goto _label)))))))))))))))))))

(event `Key|One`
  (params (Key :type "Key Structure"))
  (bind _build_preview (`self.Build Preview`))
  ; Defense inventory
  (:`Pressed`
    (set `self.Selected Defense` 0)
    (`/Game/UI/W_HUD.SetSelectedSlot` (`self.HUDRef`) 0)
    (`StaticMeshComponent.SetStaticMesh` _build_preview "/Game/Fab/Medieval_Mangonel_–_Catapult_Siege_Weapon/010_medieval_mangonel/StaticMeshes/010_medieval_mangonel.010_medieval_mangonel")
    (`SceneComponent.SetWorldScale3D` _build_preview (2.0 2.0 2.0))
    (`PrimitiveComponent.SetMaterial` _build_preview 0 "/Game/Fab/Medieval_Mangonel_–_Catapult_Siege_Weapon/010_medieval_mangonel/StaticMeshes/M.M")
    (`SceneComponent.SetVisibility` _build_preview true false)))

(event `Key|Two`
  (params (Key :type "Key Structure"))
  (bind _build_preview (`self.Build Preview`))
  ; Defense inventory
  (:`Pressed`
    (set `self.Selected Defense` 1)
    (`/Game/UI/W_HUD.SetSelectedSlot` (`self.HUDRef`) 1)
    (`StaticMeshComponent.SetStaticMesh` _build_preview "/Game/Fab/Old_Cannon_Low-poly/old_cannon/StaticMeshes/old_cannon.old_cannon")
    (`SceneComponent.SetWorldScale3D` _build_preview (15.0 15.0 15.0))
    (`PrimitiveComponent.SetMaterial` _build_preview 0 "/Game/Fab/Medieval_Mangonel_–_Catapult_Siege_Weapon/010_medieval_mangonel/StaticMeshes/M.M")
    (`SceneComponent.SetVisibility` _build_preview true false)))

(event `self.ReceiveTick`
  (params (DeltaSeconds :type "Float (single-precision)"))
  (bind _build_preview (`self.Build Preview`))
  (bind _build_preview_2 (`self.Build Preview`))
  (bind (_returnvalue _outhit) (`self.Mouse Trace`))
  (if _returnvalue
    (`self.Build Preview`
      (:`then`
        (bind (_bblockinghit _binitialoverlap _time _distance _location _impactpoint _normal _impactnormal _physmat _hitactor) (`GameplayStatics.BreakHitResult` _outhit))
        (`SceneComponent.K2_SetWorldLocation` _build_preview _impactpoint false false)
        (`SceneComponent.K2_SetWorldRotation` _build_preview (`KismetMathLibrary.MakeRotFromZ` _impactnormal) false false)
        (cast `/Game/Blueprints/BP_Tower` _hitactor
          (:`then`
            (`PrimitiveComponent.SetMaterial` _build_preview 0 "/Game/Materials/M_GhostRed.M_GhostRed"))
          (:`CastFailed`
            (cast `/Game/Defense/BP_Defense` _hitactor
              (:`then`
                (`PrimitiveComponent.SetMaterial` _build_preview 0 "/Game/Materials/M_GhostRed.M_GhostRed"))
              (:`CastFailed`
                (cast `/Game/Defense/BP_Freeze` _hitactor
                  (:`then`
                    (`PrimitiveComponent.SetMaterial` _build_preview 0 "/Game/Materials/M_GhostRed.M_GhostRed"))
                  (:`CastFailed`
                    (cast `/Game/Defense/BP_DefenseBomb` _hitactor
                      (:`then`
                        (`PrimitiveComponent.SetMaterial` _build_preview 0 "/Game/Materials/M_GhostRed.M_GhostRed" :!label _label_2))
                      (:`CastFailed`
                        (cast `/Game/Blueprints/BP_World` _hitactor
                          (:`then`
                            (bind _returnvalue_2 (`GameplayStatics.GetActorOfClass` "/Game/Blueprints/BP_Tower.BP_Tower_C"))
                            (if (> (`KismetMathLibrary.Vector_Distance` (`self.K2_GetActorLocation` _returnvalue_2) _location) 2500.0)
                              (set `self.ClosestPath` 99999.0)
                              (bind _returnvalue_3 (`GameplayStatics.GetActorOfClass` "/Game/Blueprints/BP_World.BP_World_C"))
                              (bind _path1 (`/Game/Blueprints/BP_World.Path1` _returnvalue_3))
                              (for (_array_element _array_index) _path1
                                (if (< _array_index (- (`KismetArrayLibrary.Array_Length` _path1) 1))
                                  (bind _returnvalue_4 (`KismetMathLibrary.Distance2D` (`KismetMathLibrary.Conv_VectorToVector2D` _location) (`KismetMathLibrary.Conv_VectorToVector2D` (`KismetMathLibrary.FindClosestPointOnSegment` _location _array_element (`|GetArrayItem` _path1 (+ _array_index 1))))))
                                  (if (< _returnvalue_4 (`self.ClosestPath`))
                                    (set `self.ClosestPath` _returnvalue_4))))
                              (bind _path2 (`/Game/Blueprints/BP_World.Path2` _returnvalue_3))
                              (for (_array_element_2 _array_index_2) _path2
                                (if (< _array_index_2 (- (`KismetArrayLibrary.Array_Length` _path2) 1))
                                  (bind _returnvalue_5 (`KismetMathLibrary.Distance2D` (`KismetMathLibrary.Conv_VectorToVector2D` _location) (`KismetMathLibrary.Conv_VectorToVector2D` (`KismetMathLibrary.FindClosestPointOnSegment` _location _array_element_2 (`|GetArrayItem` _path2 (+ _array_index_2 1))))))
                                  (if (< _returnvalue_5 (`self.ClosestPath`))
                                    (set `self.ClosestPath` _returnvalue_5))))
                              (bind _path3 (`/Game/Blueprints/BP_World.Path3` _returnvalue_3))
                              (for (_array_element_3 _array_index_3) _path3
                                (if (< _array_index_3 (- (`KismetArrayLibrary.Array_Length` _path3) 1))
                                  (bind _returnvalue_6 (`KismetMathLibrary.Distance2D` (`KismetMathLibrary.Conv_VectorToVector2D` _location) (`KismetMathLibrary.Conv_VectorToVector2D` (`KismetMathLibrary.FindClosestPointOnSegment` _location _array_element_3 (`|GetArrayItem` _path3 (+ _array_index_3 1))))))
                                  (if (< _returnvalue_6 (`self.ClosestPath`))
                                    (set `self.ClosestPath` _returnvalue_6))))
                              (if (> (`self.ClosestPath`) 250.0)
                                (if (< (`self.ClosestPath`) 1200.0)
                                  (if (> (`self.DefensesLeft`) 0)
                                    (switch `int` (`self.Selected Defense`)
                                      (:`0`
                                        (if (> (`/Game/Blueprints/BP_Tower.StockCatapult` _returnvalue_2) 0)
                                          (`PrimitiveComponent.SetMaterial` _build_preview_2 0 "/Game/Materials/M_GhostGreen.M_GhostGreen" :!label _label_3)
                                          (else
                                            (`PrimitiveComponent.SetMaterial` _build_preview_2 0 "/Game/Materials/M_GhostRed.M_GhostRed" :!label _label_4))))
                                      (:`1`
                                        (if (> (`/Game/Blueprints/BP_Tower.StockBomb` _returnvalue_2) 0)
                                          (goto _label_3)
                                          (else
                                            (goto _label_4))))
                                      (:`2`
                                        (if (> (`/Game/Blueprints/BP_Tower.StockFreeze` _returnvalue_2) 0)
                                          (goto _label_3)
                                          (else
                                            (goto _label_4)))))
                                    (else
                                      (`PrimitiveComponent.SetMaterial` _build_preview 0 "/Game/Materials/M_GhostGreen.M_GhostGreen")))
                                  (else
                                    (goto _label_2)))
                                (else
                                  (goto _label_2)))
                              (else
                                (goto _label_2))))
                          (:`CastFailed`
                            (goto _label_2))))))))))))
      (:`else`
        (bind _returnvalue_7 (`|AddComponentByClass` "/Script/Engine.StaticMeshComponent" false (`KismetMathLibrary.MakeTransform` _location (struct) (2.0 2.0 2.0))))
        (bind _output_get (set `self.Build Preview` _returnvalue_7))
        (`StaticMeshComponent.SetStaticMesh` _output_get "/Game/Fab/Medieval_Mangonel_–_Catapult_Siege_Weapon/010_medieval_mangonel/StaticMeshes/010_medieval_mangonel.010_medieval_mangonel")
        (`PrimitiveComponent.SetCollisionEnabled` (`self.Build Preview`) "NoCollision")
        (`PrimitiveComponent.SetMaterial` _build_preview_2 0 "/Game/Fab/Medieval_Mangonel_–_Catapult_Siege_Weapon/010_medieval_mangonel/StaticMeshes/M.M")))))

(event `Key|Three`
  (params (Key :type "Key Structure"))
  (bind _build_preview (`self.Build Preview`))
  ; Defense inventory
  (:`Pressed`
    (set `self.Selected Defense` 2)
    (`/Game/UI/W_HUD.SetSelectedSlot` (`self.HUDRef`) 2)
    (`StaticMeshComponent.SetStaticMesh` _build_preview "/Game/Fab/Woolwich_Mortar/woolwich_mortar/StaticMeshes/woolwich_mortar.woolwich_mortar")
    (`SceneComponent.SetWorldScale3D` _build_preview (60.0 60.0 60.0))
    (`PrimitiveComponent.SetMaterial` _build_preview 0 "/Game/Fab/Medieval_Mangonel_–_Catapult_Siege_Weapon/010_medieval_mangonel/StaticMeshes/M.M")
    (`SceneComponent.SetVisibility` _build_preview true false)))

(event `Key|F`
  (params (Key :type "Key Structure")))

(fn `Mouse Trace`
  (returns (ReturnValue :type Boolean) (OutHit :type "HitResult Structure"))
  (bind (_worldlocation _worlddirection) (`PlayerController.DeprojectMousePositionToWorld` (`GameplayStatics.GetPlayerController` 0)))
  (bind (_outhit _returnvalue) (`KismetSystemLibrary.LineTraceSingle` _worldlocation (+ _worldlocation (* _worlddirection 10000.0)) "TraceTypeQuery1"))
  (return _returnvalue _outhit))

(fn `RegisterKill`
  (set `self.KillsTowardReward` (+ (`self.KillsTowardReward`) 1))
  (if (>= (`self.KillsTowardReward`) 2)
    (bind _returnvalue (`GameplayStatics.GetActorOfClass` "/Game/Blueprints/BP_Tower.BP_Tower_C"))
    (set `/Game/Blueprints/BP_Tower.Gems` (+ (`/Game/Blueprints/BP_Tower.Gems` _returnvalue) 1) _returnvalue)
    (`/Game/UI/W_HUD.RefreshShop` (`self.HUDRef`))
    (set `self.KillsTowardReward` 0)))

(fn `UserConstructionScript`)
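; BP_ArcherArrow is an arrow projectile that damages defense structures it hits.
; Tick moves it straight along its forward vector at constant speed without sweeping, and it destroys itself after a short lifetime.
; Its sphere overlap runs a cast chain over DefenseBomb, FreezeCannon, Catapult and Tower, applies a fixed damage to the first match, then destroys the arrow; other actors are ignored.
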(event `self.ReceiveBeginPlay`
  (`KismetSystemLibrary.Delay` 3.0)
  (`self.K2_DestroyActor`))

(event `self.ReceiveTick`
  (params (DeltaSeconds :type "Float (single-precision)"))
  (`self.K2_AddActorWorldOffset` (* (* (`self.GetActorForwardVector`) 1500.0) DeltaSeconds)))

(event `self.Sphere.OnComponentBeginOverlap`
  (params (OverlappedComponent :type "PrimitiveComponent Object Reference") (OtherActor :type "Actor Object Reference") (OtherComp :type "PrimitiveComponent Object Reference") (OtherBodyIndex :type Integer) (bFromSweep :type Boolean) (SweepResult :type "HitResult Structure (by ref)"))
  (bind _asbp_defense_bomb (cast `/Game/Defense/BP_DefenseBomb` OtherActor)
    (:`then`
      (`/Game/Defense/BP_DefenseBomb.TakeDamage` _asbp_defense_bomb 5.0)
      (`self.K2_DestroyActor`))
    (:`CastFailed`
      (bind _asbp_freeze_cannon (cast `/Game/Defense/BP_FreezeCannon` OtherActor)
        (:`then`
          (`/Game/Defense/BP_FreezeCannon.TakeDamage` _asbp_freeze_cannon 5.0)
          (`self.K2_DestroyActor`))
        (:`CastFailed`
          (bind _asbp_catapult (cast `/Game/Defense/BP_Catapult` OtherActor)
            (:`then`
              (`/Game/Defense/BP_Catapult.TakeDamage` _asbp_catapult 5.0)
              (`self.K2_DestroyActor`))
            (:`CastFailed`
              (bind _asbp_tower (cast `/Game/Blueprints/BP_Tower` OtherActor))
              (`/Game/Blueprints/BP_Tower.ReceiveDamage` _asbp_tower 5.0)
              (`self.K2_DestroyActor`))))))))

(fn `UserConstructionScript`)
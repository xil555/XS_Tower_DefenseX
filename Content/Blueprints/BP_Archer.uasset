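; BP_Archer is a tower-defense enemy that walks waypoints from SetupArcher and destroys itself at the end.
; Tick moves it and spawns arrows on cooldown at the Tower or a catapult, though the range check measures against itself.
; FreezeEnemy pauses it temporarily; AnyDamage updates the health widget, registers kills with the player pawn and calls Die.
; A timer-based DealDamage attack and duplicated, partly disconnected movement, targeting and damage logic also remain.
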(event `FreezeEnemy`
  (set `self.bFrozen` true)
  (`KismetSystemLibrary.K2_ClearAndInvalidateTimerHandle` (`self.AttackTimer`))
  (`KismetSystemLibrary.Delay` 10.0)
  (set `self.bFrozen` false)
  (`/Engine/EditorBlueprintResources/StandardMacros.IsValid` (`self.AttackTarget`)))

(event `self.ReceiveTick`
  (params (DeltaSeconds :type "Float (single-precision)"))
  (bind _returnvalue (`self.K2_GetActorLocation`))
  (bind _shottarget (`self.ShotTarget`))
  (bind _output (`|GetArrayItem` (`self.PathPoints`) (`self.PointIndex`)))
  (bind _returnvalue_2 (`KismetMathLibrary.FindLookAtRotation` _returnvalue (`self.K2_GetActorLocation` _shottarget)))
  (if (`self.bFrozen`)
    _
    (elif (or (`self.bDead`) (`self.bReachedEnd`))
      _
      (elif (>= (`self.PointIndex`) (`KismetArrayLibrary.Array_Length` (`self.PathPoints`)))
        (set `self.bReachedEnd` true)
        (`self.K2_DestroyActor`)
        (else
          (`self.K2_SetActorLocation` (+ (`self.K2_GetActorLocation`) (* (* (`KismetMathLibrary.Normal` (- _output (`self.K2_GetActorLocation`))) (`self.MoveSpeed`)) DeltaSeconds)))
          (`self.K2_SetActorRotation` (`KismetMathLibrary.FindLookAtRotation` (`self.K2_GetActorLocation`) _output))
          (if (< (`KismetMathLibrary.Vector_Distance` (`self.K2_GetActorLocation`) _output) 60.0)
            (set `self.PointIndex` (+ (`self.PointIndex`) 1))
            (elif (<= (`self.FireCooldown`) 0.0)
              (set `self.ShotTarget` (`self.Tower`))
              (bind _outactors (`GameplayStatics.GetAllActorsOfClass` "/Game/Defense/BP_Catapult.BP_Catapult_C"))
              (for _array_element _outactors
                (if (< (`KismetMathLibrary.Vector_Distance` (`self.K2_GetActorLocation`) (`self.K2_GetActorLocation`)) (`self.ShootRange`))
                  (set `self.ShotTarget` _array_element)
                  (bind _outactors_2 (`GameplayStatics.GetAllActorsOfClass` "/Game/Defense/BP_DefenseBomb.BP_DefenseBomb_C"))
                  (for _ _outactors_2
                    _)))
              (`/Engine/EditorBlueprintResources/StandardMacros.IsValid` _shottarget
                (:`Is Valid`
                  (`self.K2_SetActorRotation` _returnvalue_2)
                  (`|SpawnActorFromClass` "/Game/Blueprints/BP_ArcherArrow.BP_ArcherArrow_C" (`KismetMathLibrary.MakeTransform` _returnvalue _returnvalue_2) "AlwaysSpawn" "MultiplyWithRoot" null null)
                  (set `self.FireCooldown` (`self.FireRate`))))
              (else
                (set `self.FireCooldown` (- (`self.FireCooldown`) DeltaSeconds))))))))))

(event `CustomEvent`
  (params (DeltaSeconds :type "Float (single-precision)"))
  (bind _returnvalue (`self.K2_GetActorLocation`))
  (bind _output (`|GetArrayItem` (`self.PathPoints`) (`self.PointIndex`)))
  (if (or (`self.bDead`) (`self.bReachedEnd`))
    _
    (elif (>= (`self.PointIndex`) (`KismetArrayLibrary.Array_Length` (`self.PathPoints`)))
      (set `self.bReachedEnd` true)
      (`self.K2_DestroyActor`)
      (else
        (`self.K2_SetActorLocation` (+ _returnvalue (* (* (`KismetMathLibrary.Normal` (- _output (`self.K2_GetActorLocation`))) (`self.MoveSpeed`)) DeltaSeconds)))
        (`self.K2_SetActorRotation` (`KismetMathLibrary.FindLookAtRotation` _returnvalue _output))
        (if (< (`KismetMathLibrary.Vector_Distance` (`self.K2_GetActorLocation`) _output) 60.0)
          (set `self.PointIndex` (+ (`self.PointIndex`) 1))
          (elif (<= (`self.FireCooldown`) 0.0)
            (set `self.ShotTarget` (`self.Tower`))
            (bind _outactors (`GameplayStatics.GetAllActorsOfClass` "/Game/Defense/BP_Catapult.BP_Catapult_C"))
            (for _array_element _outactors
              (if (< (`KismetMathLibrary.Vector_Distance` (`self.K2_GetActorLocation` _array_element) (`self.K2_GetActorLocation`)) (`self.ShootRange`))
                (set `self.ShotTarget` null)
                (break)))
            (bind _outactors_2 (`GameplayStatics.GetAllActorsOfClass` "/Game/Defense/BP_DefenseBomb.BP_DefenseBomb_C"))
            (for _array_element_2 _outactors_2
              (if (< (`KismetMathLibrary.Vector_Distance` (`self.K2_GetActorLocation`) (`self.K2_GetActorLocation` _array_element_2)) (`self.ShootRange`))
                (set `self.ShotTarget` _array_element_2)
                (break)))
            (bind _outactors_3 (`GameplayStatics.GetAllActorsOfClass` "/Game/Defense/BP_FreezeCannon.BP_FreezeCannon_C"))
            (for _array_element_3 _outactors_3
              (if (< (`KismetMathLibrary.Vector_Distance` (`self.K2_GetActorLocation` _array_element_3) (`self.K2_GetActorLocation`)) (`self.ShootRange`))
                (set `self.ShotTarget` _array_element_3)
                (break)))
            (`/Engine/EditorBlueprintResources/StandardMacros.IsValid` null)
            (else
              (set `self.FireCooldown` (- (`self.FireCooldown`) DeltaSeconds)))))))))

(event `DealDamage`
  (bind _attacktarget (`self.AttackTarget`))
  (bind _attackdamage (`self.AttackDamage`))
  (`/Engine/EditorBlueprintResources/StandardMacros.IsValid` _attacktarget
    (:`Is Valid`
      (if (`self.ActorHasTag` _attacktarget "Defense")
        (bind _asbp_freeze_cannon (cast `/Game/Defense/BP_FreezeCannon` _attacktarget)
          (:`then`
            (`/Game/Defense/BP_FreezeCannon.TakeDamage` _asbp_freeze_cannon _attackdamage))
          (:`CastFailed`
            (bind _asbp_catapult (cast `/Game/Defense/BP_Catapult` _attacktarget)
              (:`then`
                (`/Game/Defense/BP_Catapult.TakeDamage` _asbp_catapult _attackdamage))
              (:`CastFailed`
                (bind _asbp_defense_bomb (cast `/Game/Defense/BP_DefenseBomb` _attacktarget)
                  (:`then`
                    (`/Game/Defense/BP_DefenseBomb.TakeDamage` _asbp_defense_bomb (`self.AttackDamage`)))
                  (:`CastFailed`
                    (bind _asbp_tower (cast `/Game/Blueprints/BP_Tower` (`self.Tower`)))
                    (`/Game/Blueprints/BP_Tower.ReceiveDamage` _asbp_tower (`self.AttackDamage`))))))))))))

(event `CustomEvent_2`)

(event `StartAttack`
  (set `self.bReachedEnd` true)
  (`self.K2_SetActorRotation` (`self.AttackTarget`) (`KismetMathLibrary.FindLookAtRotation` (`self.K2_GetActorLocation`) (`self.K2_GetActorLocation` (`self.AttackTarget`))) false)
  (bind _returnvalue (`KismetSystemLibrary.K2_SetTimerDelegate` (delegate `DealDamage`) (`self.AttackInterval`) true))
  (set `self.AttackTimer` _returnvalue))

(event `Die`
  (set `self.bDead` true)
  (`KismetSystemLibrary.K2_ClearAndInvalidateTimerHandle` (`self.AttackTimer`))
  (cast `/Game/Blueprints/BP_Tower` (`self.Tower`))
  (`self.K2_DestroyActor`))

(event `CustomEvent_1`)

(event `self.ReceiveAnyDamage`
  (params (Damage :type "Float (single-precision)") (DamageType :type "DamageType Object Reference") (InstigatedBy :type "Controller Object Reference") (DamageCauser :type "Actor Object Reference"))
  (set `self.CurrentHealth` (- (`self.CurrentHealth`) Damage))
  (bind _aswbp_archer_health (cast `/Game/UI/WBP_ArcherHealth` (`WidgetComponent.GetUserWidgetObject` (`self.Widget`))))
  (`/Game/UI/WBP_ArcherHealth.SetHealthPercent` _aswbp_archer_health (/ (`self.CurrentHealth`) (`self.MaxHealth`)))
  (if (<= (`self.CurrentHealth`) 0.0)
    (bind _asbp_player_pawn (cast `/Game/Blueprints/BP_PlayerPawn` (`GameplayStatics.GetPlayerPawn` 0)))
    (`/Game/Blueprints/BP_PlayerPawn.RegisterKill` _asbp_player_pawn)
    (`self.Die`)))

(event `CustomEvent_3`
  (set `self.bDead` true)
  (`KismetSystemLibrary.K2_ClearAndInvalidateTimerHandle` (`self.AttackTimer`))
  (cast `/Game/Blueprints/BP_Tower` (`self.Tower`))
  (`self.K2_DestroyActor`))

(event `CustomEvent_4`
  (params (Damage :type "Float (single-precision)") (DamageType :type "DamageType Object Reference") (InstigatedBy :type "Controller Object Reference") (DamageCauser :type "Actor Object Reference"))
  (set `self.CurrentHealth` (- (`self.CurrentHealth`) Damage))
  (bind _aswbp_archer_health (cast `/Game/UI/WBP_ArcherHealth` (`WidgetComponent.GetUserWidgetObject` (`self.Widget`))))
  (`/Game/UI/WBP_ArcherHealth.SetHealthPercent` _aswbp_archer_health (/ (`self.CurrentHealth`) (`self.MaxHealth`)))
  (if (<= (`self.CurrentHealth`) 0.0)
    (`self.Die`)))

(event `self.ReceiveBeginPlay`
  (set `self.CurrentHealth` (`self.MaxHealth`)))

(event `CustomEvent_5`
  (set `self.CurrentHealth` (`self.MaxHealth`)))

(fn `ReceiveDamage`
  (params (Amount :type "Float (double-precision)"))
  (set `self.CurrentHealth` (- (`self.CurrentHealth`) Amount))
  (bind _aswbp_archer_health (cast `/Game/UI/WBP_ArcherHealth` (`WidgetComponent.GetUserWidgetObject` (`self.Widget`))))
  (`/Game/UI/WBP_ArcherHealth.SetHealthPercent` _aswbp_archer_health 1.0)
  (if (<= (`self.CurrentHealth`) 0.0)
    (`self.Die`)))

(fn `SetupArcher`
  (params (InPoints :type "Array of Vector Structure") (`InTower ` :type "Actor Object Reference"))
  (set `self.PathPoints` InPoints)
  (set `self.Tower` `InTower `)
  (set `self.AttackTarget` (`self.Tower`))
  (set `self.CurrentHealth` (`self.MaxHealth`))
  (set `self.PointIndex` 0)
  (set `self.bReachedEnd` false)
  (`SkeletalMeshComponent.PlayAnimation` (`self.Archer`) "/Game/Characters/Archer/Standing_Aim_Walk_Forward_Anim.Standing_Aim_Walk_Forward_Anim" true)
  (set `self.bDead` false)
  (`self.K2_SetActorLocation` (`|GetArrayItem` (`self.PathPoints`)))
  (bind _aswbp_archer_health (cast `/Game/UI/WBP_ArcherHealth` (`WidgetComponent.GetUserWidgetObject` (`self.Widget`))))
  (`/Game/UI/WBP_ArcherHealth.SetHealthPercent` _aswbp_archer_health 1.0)
  (`self.K2_SetActorRotation` (`KismetMathLibrary.FindLookAtRotation` (`self.K2_GetActorLocation`) (`self.K2_GetActorLocation` (`self.Tower`)))))

(fn `UserConstructionScript`)
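; Sand worm tower-defense enemy that follows supplied path points to the tower, deals eruption damage there and dies.
; Tick drives movement and records nearby catapults as AttackTarget without attacking them; FreezeEnemy pauses Tick logic temporarily.
; Random timers alternate burrowing and surfacing, toggling visibility and collision, with ReceiveDamage ignored underground.
; AnyDamage registers player kills but zeroes health whenever the health widget cast succeeds, while ReceiveDamage casts to the mummy's widget class.
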(event `FreezeEnemy`
  (set `self.bFrozen` true)
  (set `self.MoveSpeed` 0.0)
  (`KismetSystemLibrary.Delay` 10.0)
  (set `self.bFrozen` false)
  (set `self.MoveSpeed` (`self.MoveSpeed`)))

(event `self.ReceiveTick`
  (params (DeltaSeconds :type "Float (single-precision)"))
  (bind _returnvalue (`self.K2_GetActorLocation`))
  (bind _output (`|GetArrayItem` (`self.PathPoints`) (`self.PointIndex`)))
  (bind _returnvalue_2 (+ (* (`KismetMathLibrary.Normal` (- _output (`self.K2_GetActorLocation`))) (`self.MoveSpeed`) (`GameplayStatics.GetWorldDeltaSeconds`)) (`self.K2_GetActorLocation`)))
  (if (`self.bFrozen`)
    _
    (elif (not (or (`self.bDead`) (`self.bReachedEnd`)))
      (bind _outactors (`GameplayStatics.GetAllActorsOfClass` "/Game/Defense/BP_Catapult.BP_Catapult_C"))
      (for _array_element _outactors
        (if (< (`KismetMathLibrary.Vector_Distance` (`self.K2_GetActorLocation`) (`self.K2_GetActorLocation` _array_element)) (`self.DefenseDetectRange`))
          (`/Engine/EditorBlueprintResources/StandardMacros.IsValid` (`self.AttackTarget`)
            (:`Is Not Valid`
              (set `self.AttackTarget` _array_element)))))
      (if (>= (`self.PointIndex`) (`KismetArrayLibrary.Array_Length` (`self.PathPoints`)))
        (set `self.AttackTarget` (`self.Tower`))
        (`self.DeliverFinalAttack`)
        (else
          (`self.K2_SetActorLocation` _returnvalue_2)
          (`self.K2_SetActorRotation` (`KismetMathLibrary.FindLookAtRotation` _returnvalue (+ _returnvalue (* (* (`KismetMathLibrary.Normal` (- (`|GetArrayItem` (`self.PathPoints`) (`self.PointIndex`)) (`self.K2_GetActorLocation`))) (`self.MoveSpeed`)) DeltaSeconds))))
          (if (< (`KismetMathLibrary.Vector_Distance` _returnvalue_2 _output) 60.0)
            (set `self.PointIndex` (+ (`self.PointIndex`) 1))))))))

(event `StartAttack`)

(event `GoUnderground`
  (if (not (or (`self.bDead`) (`self.bReachedEnd`)))
    (set `self.bUnderground ` true)
    (`self.ApplyVisibility `)
    (`self.ScheduleNextSurface `)))

(event `ComeToSurface`
  (if (not (or (`self.bDead`) (`self.bReachedEnd`)))
    (set `self.bUnderground ` false)
    (`self.ApplyVisibility `)
    (`self.ScheduleNextBurrow `)))

(event `OnBurrowTimer`
  (`self.GoUnderground`))

(event `ScheduleNextBurrow`
  (bind _returnvalue (`KismetSystemLibrary.K2_SetTimerDelegate` (delegate `OnBurrowTimer`) (`KismetMathLibrary.RandomFloatInRange` (`self.MinBurrowTime `) (`self.MaxBurrowTime`))))
  (set `self.BurrowTimer ` _returnvalue))

(event `OnSurfaceTimer`
  (`self.ComeToSurface`))

(event `ScheduleNextSurface`
  (bind _returnvalue (`KismetSystemLibrary.K2_SetTimerDelegate` (delegate `OnSurfaceTimer`) (`KismetMathLibrary.RandomFloatInRange` (`self.MinBurrowTime `) (`self.MaxBurrowTime`))))
  (set `self.BurrowTimer ` _returnvalue))

(event `self.ReceiveAnyDamage`
  (params (Damage :type "Float (single-precision)") (DamageType :type "DamageType Object Reference") (InstigatedBy :type "Controller Object Reference") (DamageCauser :type "Actor Object Reference"))
  (set `self.CurrentHealth` (- (`self.CurrentHealth`) Damage))
  (bind _aswbp_sand_worm_health (cast `/Game/UI/WBP_SandWormHealth` (`WidgetComponent.GetUserWidgetObject` (`self.HealthWidget`)))
    (:`then`
      (set `self.CurrentHealth` 0.0)
      (`/Game/UI/WBP_SandWormHealth.SetHealthPercent` _aswbp_sand_worm_health (/ (`self.CurrentHealth`) (`self.MaxHealth`))))
    (:`CastFailed`
      _))
  (if (<= (`self.CurrentHealth`) 0.0)
    (bind _asbp_player_pawn (cast `/Game/Blueprints/BP_PlayerPawn` (`GameplayStatics.GetPlayerPawn` 0)))
    (`/Game/Blueprints/BP_PlayerPawn.RegisterKill` _asbp_player_pawn)
    (`self.Die`)))

(event `self.ReceiveBeginPlay`
  (set `self.CurrentHealth` (`self.MaxHealth`)))

(event `DeliverFinalAttack`
  (set `self.bReachedEnd` true)
  (`KismetSystemLibrary.K2_ClearAndInvalidateTimerHandle` (`self.BurrowTimer `))
  (set `self.bUnderground ` false)
  (`self.ApplyVisibility `)
  (`/Engine/EditorBlueprintResources/StandardMacros.IsValid` (`self.Tower`)
    (:`Is Valid`
      (if true
        (bind _asbp_tower (cast `/Game/Blueprints/BP_Tower` (`self.Tower`)))
        (`/Game/Blueprints/BP_Tower.ReceiveDamage` _asbp_tower (`self.EruptDamage`))
        (`self.Die`)))))

(event `Die`
  (set `self.bDead` true)
  (`KismetSystemLibrary.K2_ClearAndInvalidateTimerHandle` (`self.BurrowTimer `))
  (cast `/Game/Blueprints/BP_Tower` (`self.Tower`))
  (`self.K2_DestroyActor`))

(event `DealDamage`)

(fn `ApplyVisibility `
  (bind _sandworm (`self.SandWorm`))
  (bind _healthwidget (`self.HealthWidget`))
  (bind _sandworm_2 (`self.SandWorm`))
  (bind _healthwidget_2 (`self.HealthWidget`))
  (if (`self.bUnderground `)
    (`SceneComponent.SetVisibility` _sandworm_2 false true)
    (`SceneComponent.SetVisibility` _healthwidget_2 false true)
    (`PrimitiveComponent.SetCollisionEnabled` _healthwidget_2 "NoCollision")
    (`PrimitiveComponent.SetCollisionEnabled` _sandworm_2 "NoCollision")
    (else
      (`SceneComponent.SetVisibility` _sandworm true true)
      (`SceneComponent.SetVisibility` _healthwidget true true)
      (`PrimitiveComponent.SetCollisionEnabled` _sandworm "QueryAndPhysics")
      (`PrimitiveComponent.SetCollisionEnabled` _healthwidget "QueryAndPhysics"))))

(fn `ReceiveDamage`
  (params (Amount :type "Float (double-precision)"))
  (if (or (`self.bUnderground `) (`self.bDead`))
    (return)
    (else
      (set `self.CurrentHealth` (- (`self.CurrentHealth`) Amount))
      (bind _aswbp_mummy_health (cast `/Game/UI/WBP_MummyHealth` (`WidgetComponent.GetUserWidgetObject` (`self.HealthWidget`))))
      (`/Game/UI/WBP_MummyHealth.SetHealthPercent` _aswbp_mummy_health (/ (`self.CurrentHealth`) (`self.MaxHealth`)))
      (if (<= (`self.CurrentHealth`) 0.0)
        (`self.Die`)))))

(fn `SetupWorm`
  (params (InPoints :type "Array of Vector Structure") (`InTower ` :type "Actor Object Reference"))
  (set `self.PathPoints` InPoints)
  (set `self.Tower` `InTower `)
  (set `self.CurrentHealth` (`self.MaxHealth`))
  (set `self.PointIndex` 0)
  (set `self.bReachedEnd` false)
  (set `self.bDead` false)
  (set `self.bUnderground ` false)
  (`self.ApplyVisibility `)
  (`SkeletalMeshComponent.PlayAnimation` (`self.SandWorm`) "/Game/Fab/Fat_Worm_FREE/worm_free_fab_Anim.worm_free_fab_Anim" true)
  (`self.K2_SetActorLocation` (`|GetArrayItem` (`self.PathPoints`)))
  (bind _aswbp_sand_worm_health (cast `/Game/UI/WBP_SandWormHealth` (`WidgetComponent.GetUserWidgetObject` (`self.HealthWidget`))))
  (`/Game/UI/WBP_SandWormHealth.SetHealthPercent` _aswbp_sand_worm_health 1.0)
  (`self.K2_SetActorRotation` (`KismetMathLibrary.FindLookAtRotation` (`self.K2_GetActorLocation`) (`self.K2_GetActorLocation` (`self.Tower`))))
  (`self.ScheduleNextBurrow `))

(fn `UserConstructionScript`)
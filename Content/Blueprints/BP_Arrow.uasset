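; BP_Arrow is a homing projectile that flies toward an assigned Target actor.
; Each tick it steps along the normalized direction to the target at Speed, without sweep, and rotates to face it.
; It limits its life with Lifetime and destroys itself once the target is no longer valid.
; It has no overlap or hit handling of its own.
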(event `self.ReceiveBeginPlay`
  (`self.SetLifeSpan` (`self.Lifetime`)))

(event `self.ReceiveTick`
  (params (DeltaSeconds :type "Float (single-precision)"))
  (bind _returnvalue (`self.K2_GetActorLocation`))
  (bind _returnvalue_2 (`self.K2_GetActorLocation` (`self.Target`)))
  (`/Engine/EditorBlueprintResources/StandardMacros.IsValid` (`self.Target`)
    (:`Is Valid`
      (if true
        (bind _output_get (set `self.Dir` (`KismetMathLibrary.Normal` (- _returnvalue_2 _returnvalue))))
        (set `self.MoveStep` (* _output_get (* (`self.Speed`) DeltaSeconds)))
        (`self.K2_SetActorLocation` (+ (`self.K2_GetActorLocation`) (`self.MoveStep`)))
        (`self.K2_SetActorRotation` (`KismetMathLibrary.FindLookAtRotation` _returnvalue _returnvalue_2))))
    (:`Is Not Valid`
      (`self.K2_DestroyActor`))))

(fn `UserConstructionScript`)
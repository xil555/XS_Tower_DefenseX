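; Adaptive music director actor that layers four audio stems to match the danger around the tower.
; A looping timer recomputes a 0–1 intensity from tower damage, capped mummy count and a wave term, with a low fallback when no tower exists.
; Intensity drives stem volumes: the drone recedes as percussion, tense and pulse layers fade in over staggered thresholds.
; SessionBias is randomized at start but unused here, and WaveTerm is never set here.
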(event `RefreshMusic`
  (`self.ComputeIntensity`)
  (`self.ApplyStemMix`))

(event `self.ReceiveBeginPlay`
  (`self.FindTower`)
  (`self.StartMusic`)
  (`KismetSystemLibrary.K2_SetTimer` null "RefreshMusic" (`self.UpdateInterval`) true))

(fn `ApplyStemMix`
  (bind _output_get (set `self.VolDrone` (`KismetMathLibrary.Lerp` 0.55 0.25 (`self.Intensity`))))
  (bind _output_get_2 (set `self.VolPerc` (* (`KismetMathLibrary.FClamp` (/ (- (`self.Intensity`) 0.25) 0.35)) 0.55)))
  (bind _output_get_3 (set `self.VolTense` (* (`KismetMathLibrary.FClamp` (/ (- (`self.Intensity`) 0.55) 0.3)) 0.65)))
  (bind _output_get_4 (set `self.VolPulse` (* (`KismetMathLibrary.FClamp` (/ (- (`self.Intensity`) 0.8) 0.2)) 0.75)))
  (`AudioComponent.SetVolumeMultiplier` (`self.AC_Drone `) _output_get)
  (`AudioComponent.SetVolumeMultiplier` (`self.AC_Percussion `) _output_get_2)
  (`AudioComponent.SetVolumeMultiplier` (`self.AC_Tense `) _output_get_3)
  (`AudioComponent.SetVolumeMultiplier` (`self.AC_Pulse `) _output_get_4))

(fn `ComputeIntensity`
  (bind _towerref (`self.TowerRef`))
  (`self.FindTower`)
  (`/Engine/EditorBlueprintResources/StandardMacros.IsValid` _towerref
    (:`Is Valid`
      (bind _count (`self.CountEnemies`))
      (set `self.Intensity` (`KismetMathLibrary.FClamp` (+ (* (- 1.0 (/ (`/Game/Blueprints/BP_Tower.CurrentHealth` _towerref) (`/Game/Blueprints/BP_Tower.MaxHealth` _towerref))) 0.35) (* (`KismetMathLibrary.FMin` (/ (`KismetMathLibrary.Conv_IntToDouble` _count) (`self.EnemyPressureCap`)) 1.0) 0.4) (`self.WaveTerm`)))))
    (:`Is Not Valid`
      (set `self.Intensity` 0.2))))

(fn `CountEnemies`
  (returns (Count :type Integer))
  (bind _outactors (`GameplayStatics.GetAllActorsOfClass` "/Game/Blueprints/BP_Mummy.BP_Mummy_C"))
  (return (`KismetArrayLibrary.Array_Length` _outactors)))

(fn `FindTower`
  (bind _returnvalue (`GameplayStatics.GetActorOfClass` "/Game/Blueprints/BP_Tower.BP_Tower_C"))
  (set `self.TowerRef` _returnvalue))

(fn `StartMusic`
  (set `self.SessionBias` (`KismetMathLibrary.RandomFloatInRange` -1.0 1.0))
  (`AudioComponent.SetVolumeMultiplier` (`self.AC_Drone `) 0.0)
  (`AudioComponent.SetVolumeMultiplier` (`self.AC_Percussion `) 0.0)
  (`AudioComponent.SetVolumeMultiplier` (`self.AC_Tense `) 0.0)
  (`AudioComponent.SetVolumeMultiplier` (`self.AC_Pulse `) 0.0)
  (`self.ComputeIntensity`)
  (`self.ApplyStemMix`))

(fn `StopMusic`
  (`AudioComponent.Stop` (`self.AC_Drone `))
  (`AudioComponent.Stop` (`self.AC_Percussion `))
  (`AudioComponent.Stop` (`self.AC_Tense `))
  (`AudioComponent.Stop` (`self.AC_Pulse `)))

(fn `UserConstructionScript`)